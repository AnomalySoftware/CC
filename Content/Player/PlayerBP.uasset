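; Player character for a 2D wave-based melee game, with flying X/Z movement, a cursor-aimed sword arm, slash, cooldown-limited lunge and bomb spawning.
; Attack flags gate sword-overlap damage to enemies, while Tick interpolates sword swing and lunge speed and updates flipbooks and facing.
; Tick also checks GameInstance wave kills to clear enemies and open the shop, or loads GAME_OVER on death.
; Hat and sword skins come from the GameInstance.
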(event OnComponentBeginOverlap(SwordHitbox)
  (params (OverlappedComponent :type Primitive%20Component%20Object%20Reference) (OtherActor :type Actor%20Object%20Reference) (OtherComp :type Primitive%20Component%20Object%20Reference) (OtherBodyIndex :type Integer) (bFromSweep :type Boolean) (SweepResult :type Hit%20Result%20Structure%20%28by%20ref%29))
  ;[1 1 1] Sword Damage
  (if (not (Variables|Default|GetshopOpen))
    (if (Variables|Default|GetAlive)
      (if (or (Variables|Default|GetAttacking) (Variables|Default|GetLunging))
        (bind _asenemy_base_bp (Utilities|Casting|CastToEnemyBaseBP OtherActor)
          (:then
            (Audio|PlaySound2D "/Game/Sound/Hit.Hit" 1.0 1.0 0.0 0 0)
            (if (Variables|Default|GetLunging)
              (Variables|/Game/Enemy/EnemyBaseBP.EnemyBaseBP_C|SetHealth _asenemy_base_bp (- (Variables|/Game/Enemy/EnemyBaseBP.EnemyBaseBP_C|GetHealth _asenemy_base_bp) 20))
              (else
                (Variables|/Game/Enemy/EnemyBaseBP.EnemyBaseBP_C|SetHealth _asenemy_base_bp (- (Variables|/Game/Enemy/EnemyBaseBP.EnemyBaseBP_C|GetHealth _asenemy_base_bp) 10)))))
          (:CastFailed
            (Development|PrintString "Cast failed")))))))

(event EventBeginPlay
  ;[1 1 1] Startup
  (bind _returnvalue (UserInterface|CreateWidget "/Game/GUI/PlayerStat.PlayerStat_C"))
  (UserInterface|Viewport|AddtoViewport _returnvalue 0)
  (Rendering|SetVisibility (Variables|Default|GetHat) false false)
  (Utilities|FlowControl|Delay 0.2)
  (CallFunction|SetHat)
  (CallFunction|SetSword)
  (Variables|Default|SetShopGUI 0))

(event EventTick
  (params (DeltaSeconds :type Float%20%28single-precision%29))
  (bind _returnvalue (Transformation|GetActorLocation))
  (bind _returnvalue_2 (Game|GetPlayerController 0))
  (bind _returnvalue_3 (Game|GetGameInstance))
  (bind _mouselocation (Variables|Default|GetMouseLocation))
  (bind _playerarm (Variables|Default|GetPlayerArm))
  (bind _sprite (Variables|Default|GetSprite))
  (bind _maxhealth (Variables|Default|GetMaxHealth))
  (bind _returnvalue_4 (Math|Rotator|FindLookatRotation _returnvalue _mouselocation))
  (bind _asccgame_instance (Utilities|Casting|CastToCCGameInstance _returnvalue_3))
  (if (and (== (stale Input|AxisEvents|InputAxisMoveX AxisValue) 0.0) (== (stale Input|AxisEvents|InputAxisMoveY AxisValue) 0.0))
    (Sprite|SetFlipbook (Variables|Default|GetSprite) "/Game/Player/PlayerMedia/Player1_FB.Player1_FB"))
  (Variables|/Game/Engine/CCGameInstance.CCGameInstance_C|SetWaveKillsNeeded _asccgame_instance (+ (* (Variables|/Game/Engine/CCGameInstance.CCGameInstance_C|GetWave _asccgame_instance) 5) 5))
  (Transformation|SetWorldLocation (Variables|Default|GetWidget) (Variables|Default|GetMouseLocation) false false)
  (if (> (Variables|Default|GetHealth) 0)
    (if (> (Variables|Default|GetHealth) _maxhealth)
      (Variables|Default|SetHealth _maxhealth))
    (Variables|Default|SetLungeCoolDown (Math|Interpolation|FInterptoConstant (Variables|Default|GetLungeCoolDown) 1.0 (Utilities|Time|GetWorldDeltaSeconds) 1.0))
    (Variables|/Script/Engine.CharacterMovementComponent|SetMaxFlySpeed (Variables|Character|GetCharacterMovement) (Math|Interpolation|FInterpTo (Variables|/Script/Engine.CharacterMovementComponent|GetMaxFlySpeed (Variables|Character|GetCharacterMovement)) 1.5e+02 (Utilities|Time|GetWorldDeltaSeconds) 3.0))
    (Variables|Default|SetSwordRotation (Math|Interpolation|FInterpTo (Variables|Default|GetSwordRotation) 9e+01 (Utilities|Time|GetWorldDeltaSeconds) 6.0))
    (Transformation|SetRelativeRotation (Variables|Default|GetPlayerSword) (Math|Rotator|MakeRotator 0.0 (Variables|Default|GetSwordRotation) 0.0) false false)
    (if (Variables|Default|GetLunging)
      (Pawn|Input|AddMovementInput (Variables|Default|GetLungeForwardVector) 1.0 false))
    (if (>= (.x (Variables|Default|GetMouseLocation)) (.x (Transformation|GetActorLocation)))
      (Transformation|SetRelativeScale3D _sprite "1.000000,1.000000,1.000000")
      (Transformation|SetRelativeRotation _playerarm (Math|Rotator|MakeRotator 0.0 (* (+ (.pitch _returnvalue_4) 9e+01) -1.0) 0.0) false false)
      (else
        (Transformation|SetRelativeScale3D _sprite "-1.000000,1.000000,1.000000")
        (Transformation|SetRelativeRotation _playerarm (Math|Rotator|MakeRotator 0.0 (* (+ (.pitch _returnvalue_4) 9e+01) -1.0) 0.0) false false)))
    (if (== (Math|Vector|VectorLength (Transformation|GetVelocity)) 0.0)
      ;[0.000804 0 0.09271] FlipBooks
      (Sprite|SetFlipbook (Variables|Default|GetSprite) "/Game/Player/PlayerMedia/Player1_FB.Player1_FB")
      (Transformation|SetRelativeLocation (Variables|Default|GetPlayerArm) "-4.000000,1.000000,6.000000" false false)
      (elif (Variables|Default|GetLunging)
        (Sprite|SetFlipbook (Variables|Default|GetSprite) "/Game/Player/PlayerMedia/PlayerLunge_FB.PlayerLunge_FB")
        (Transformation|SetRelativeLocation (Variables|Default|GetPlayerArm) "-4.000000,1.000000,4.000000" false false)
        (else
          (Sprite|SetFlipbook (Variables|Default|GetSprite) "/Game/Player/PlayerMedia/PlayerRun_FB.PlayerRun_FB")
          (Transformation|SetRelativeLocation (Variables|Default|GetPlayerArm) "-4.000000,1.000000,6.000000" false false))))
    (if (>= (Variables|/Game/Engine/CCGameInstance.CCGameInstance_C|GetWaveKills (.AsCCGame%20Instance (Utilities|Casting|CastToCCGameInstance (Game|GetGameInstance)))) (Variables|/Game/Engine/CCGameInstance.CCGameInstance_C|GetWaveKillsNeeded (.AsCCGame%20Instance (Utilities|Casting|CastToCCGameInstance (Game|GetGameInstance)))))
      ;[0.1844 0.09098 0.01206] Open Shop
      (if (not (Variables|Default|GetshopOpen))
        (Variables|Default|SetwaveEnded true)
        (bind _outactors (Actor|GetAllActorswithTag "Enemy"))
        (for _array_element _outactors
          (Actor|DestroyActor _array_element))
        (if (not (Variables|Default|GetshopOpen))
          (Variables|/Script/Engine.PlayerController|SetbShowMouseCursor _returnvalue_2 true)
          (Variables|Default|SetshopOpen true)
          (bind _returnvalue_5 (UserInterface|CreateWidget "/Game/GUI/Shop/ShopGUI.ShopGUI_C" _returnvalue_2))
          (UserInterface|Viewport|AddtoViewport _returnvalue_5 0)
          (Variables|Default|SetShopGUI _returnvalue_5)))
      (else
        (Variables|/Script/Engine.PlayerController|SetbShowMouseCursor (Game|GetPlayerController 0) false)))
    (else
      (Variables|Default|SetHealth 0)
      (Utilities|FlowControl|DoOnce false
        (:Completed
          ;[0.101 0.01669 0] Game Over
          (Variables|Default|SetAlive false)
          (bind _outactors_2 (Actor|GetAllActorswithTag "Enemy"))
          (for _array_element_2 _outactors_2
            (Actor|DestroyActor _array_element_2))
          (Utilities|FlowControl|Delay 0.1)
          (Game|OpenLevel(byName) "GAME_OVER"))))))

(event Input|ActionEvents|InputActionLunge
  (params (Key :type Key%20Structure))
  ;[0.06834 0.1927 0.04798] Lunge
  (:Pressed
    (if (Variables|Default|GetAlive)
      (if (>= (Variables|Default|GetLungeCoolDown) 1.0)
        (if (not (Variables|Default|GetLunging))
          (Variables|Default|SetLunging true)
          (Variables|Default|SetSwordRotation 1.8e+02)
          (Variables|Default|SetLungeForwardVector (Math|Vector|GetForwardVector (Math|Rotator|FindLookatRotation (Transformation|GetActorLocation) (Variables|Default|GetMouseLocation))))
          (Variables|/Script/Engine.CharacterMovementComponent|SetMaxFlySpeed (Variables|Character|GetCharacterMovement) (Variables|Default|GetLungeDistance))
          (Variables|Default|SetLungeCoolDown 0.0)
          (Components|Activation|Activate (Variables|Default|GetSparks) true)
          (Class|PlayerController|ClientPlayCameraShake (Game|GetPlayerController 0) "/Game/Shakes/HeavyShake.HeavyShake_C" 1.0 "CameraLocal" "0, 0, 0")
          (Audio|PlaySound2D "/Game/Sound/Lunge_Sound.Lunge_Sound" 1.0 1.0 0.0 0 0)
          (Utilities|FlowControl|Delay 0.6)
          (Variables|Default|SetLunging false))))))

(event Input|ActionEvents|InputActionSlash
  (params (Key :type Key%20Structure))
  ;[1 1 1] Startup
  (:Pressed
    (if (not (Variables|Default|GetshopOpen))
      (if (Variables|Default|GetAlive)
        (if (not (Variables|Default|GetLunging))
          (if (not (Variables|Default|GetAttacking))
            (Variables|Default|SetAttacking true)
            (Variables|Default|SetSwordRotation 1.8e+02)
            (Class|PlayerController|ClientPlayCameraShake (Game|GetPlayerController 0) "/Game/Shakes/SlightShake.SlightShake_C" 1.0 "CameraLocal" "0, 0, 0")
            (Audio|PlaySound2D "/Game/Sound/Slash_Sound3.Slash_Sound3" 1.0 1.0 0.0 0 0)
            (Utilities|FlowControl|Delay 0.15)
            (Variables|Default|SetAttacking false)))))))

(event Input|AxisEvents|InputAxisMoveX
  (params (AxisValue :type Float%20%28single-precision%29))
  (if (not (Variables|Default|GetshopOpen))
    ;[1 1 1] WASD
    (if (Variables|Default|GetAlive)
      (if (not (Variables|Default|GetLunging))
        (Pawn|Input|AddMovementInput "1.000000, 0, 0" (* AxisValue (Variables|Default|GetSpeed)) false)))))

(event Input|AxisEvents|InputAxisMoveY
  (params (AxisValue :type Float%20%28single-precision%29))
  (if (not (Variables|Default|GetshopOpen))
    ;[1 1 1] WASD
    (if (Variables|Default|GetAlive)
      (if (not (Variables|Default|GetLunging))
        (Pawn|Input|AddMovementInput "0.000000, 0,1.000000" AxisValue false)))))

(event Input|AxisEvents|InputAxisMouseX
  (params (AxisValue :type Float%20%28single-precision%29))
  (bind _returnvalue (Transformation|GetActorLocation))
  (if (not (Variables|Default|GetshopOpen))
    ;[1 1 1] MouseControl
    (if (Variables|Default|GetAlive)
      (if (Variables|Default|GetusingController)
        (Variables|Default|SetMouseX (+ AxisValue 25.0))
        (else
          (bind _output_get (Variables|Default|SetMouseX (+ AxisValue (Variables|Default|GetMouseX))))
          (Variables|Default|SetMouseLocation (Math|Vector|MakeVector (+ _output_get (.x _returnvalue)) (.y _returnvalue) (+ (.z _returnvalue) (stale Input|AxisEvents|InputAxisMouseY _output_get)))))))))

(event Input|AxisEvents|InputAxisMouseY
  (params (AxisValue :type Float%20%28single-precision%29))
  (bind _returnvalue (Transformation|GetActorLocation))
  ;[1 1 1] MouseControl
  (if (not (Variables|Default|GetshopOpen))
    (if (Variables|Default|GetAlive)
      (if (Variables|Default|GetusingController)
        (Variables|Default|SetMouseY (+ AxisValue -15.0))
        (else
          (bind _output_get (Variables|Default|SetMouseY (+ AxisValue (Variables|Default|GetMouseY))))))
      (Variables|Default|SetMouseLocation (Math|Vector|MakeVector (+ (stale Input|AxisEvents|InputAxisMouseX _output_get) (.x _returnvalue)) (.y _returnvalue) (+ (.z _returnvalue) _output_get))))))

(event Input|KeyboardEvents|E
  (params (Key :type Key%20Structure))
  (:Pressed
    (Variables|Default|SetusingController false)))

(event Input|KeyboardEvents|X
  (params (Key :type Key%20Structure))
  (bind _returnvalue (Transformation|GetActorLocation))
  ;[1 1 1] Spawn Bomb
  (:Released
    (Game|SpawnActorfromClass "/Game/Items/Bomb/Bomb_BP.Bomb_BP_C" (Math|Transform|MakeTransform (Math|Vector|MakeVector (.x _returnvalue) (.y _returnvalue) (.z _returnvalue)) "0, 0, 0" "1,1,1") "Undefined" 0 0)))

(fn ConstructionScript)

(fn SetHat
  (bind _hat (Variables|Default|GetHat))
  (bind _asccgame_instance (Utilities|Casting|CastToCCGameInstance (Game|GetGameInstance)))
  (Rendering|Components|Sprite|SetSprite _hat (Utilities|ResolveSoftReference (Variables|/Game/Engine/CCGameInstance.CCGameInstance_C|Gethat _asccgame_instance)))
  (Rendering|SetVisibility _hat true false))

(fn SetSword
  (bind _asccgame_instance (Utilities|Casting|CastToCCGameInstance (Game|GetGameInstance)))
  (Rendering|Components|Sprite|SetSprite (Variables|Default|GetPlayerSword) (Utilities|ResolveSoftReference (Variables|/Game/Engine/CCGameInstance.CCGameInstance_C|GetswordSkin _asccgame_instance))))