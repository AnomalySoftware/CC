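; EnemyBaseBP is an enemy base Blueprint that provides a hit flash and spawn counting.
; HitMat_Event swaps the Sprite's material to White, then restores Lit_Spr after a brief delay.
; The construction script increments EnemySpawns on CCGameInstance for every instance except Thorn_BP, so the count changes whenever construction runs.
; The Flash function is an empty stub.
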(event Custom|HitMat_Event
  (bind _sprite (Variables|Default|GetSprite))
  (Rendering|Material|SetMaterial _sprite 0 "/Game/Effects/Materials/White.White")
  (Utilities|FlowControl|Delay 0.1)
  (Rendering|Material|SetMaterial _sprite 0 "/Game/Effects/Materials/Lit_Spr.Lit_Spr"))

(fn ConstructionScript
  (bind _returnvalue (Game|GetGameInstance))
  (bind _asccgame_instance (Utilities|Casting|CastToCCGameInstance _returnvalue))
  (Utilities|Casting|CastToThorn_BP self
    (:CastFailed
      (Variables|/Game/Engine/CCGameInstance.CCGameInstance_C|SetEnemySpawns _asccgame_instance (+ (Variables|/Game/Engine/CCGameInstance.CCGameInstance_C|GetEnemySpawns _asccgame_instance) 1)))))

(fn Flash)