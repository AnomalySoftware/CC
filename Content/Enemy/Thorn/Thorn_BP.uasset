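; Thorn_BP is an enemy thorn hazard that plays a one-shot sprite animation and sound on spawn, then damages the player if they are standing in it.
; Begin and end overlap events track whether PlayerBP is inside through a flag.
; BeginPlay waits briefly, subtracts health directly from the player pawn if the flag is set, then destroys the actor after a second delay.
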(event EventBeginPlay
  (bind _returnvalue (Game|Player|GetPlayerPawn 0))
  (bind _asplayer_bp (Utilities|Casting|CastToPlayerBP _returnvalue))
  (Audio|PlaySound2D "/Game/Enemy/Thorn/thornjump.thornjump" 1.0 1.0 0.0 0 0)
  (Components|Timeline|SetLooping (Variables|Default|GetSprite) false)
  (Utilities|FlowControl|Delay 0.32)
  (if (Variables|Default|GetOverlap)
    (Variables|/Game/Player/PlayerBP.PlayerBP_C|SetHealth _asplayer_bp (- (Variables|/Game/Player/PlayerBP.PlayerBP_C|GetHealth _asplayer_bp) 5)))
  (Utilities|FlowControl|Delay 0.7)
  (Actor|DestroyActor))

(event Collision|EventActorBeginOverlap
  (params (OtherActor :type Actor%20Object%20Reference))
  (Utilities|Casting|CastToPlayerBP OtherActor)
  (Variables|Default|SetOverlap true))

(event Collision|EventActorEndOverlap
  (params (OtherActor :type Actor%20Object%20Reference))
  (Utilities|Casting|CastToPlayerBP OtherActor)
  (Variables|Default|SetOverlap false))

(fn ConstructionScript
  (|CallParentFunction))